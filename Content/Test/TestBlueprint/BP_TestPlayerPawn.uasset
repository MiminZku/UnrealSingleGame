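; Test player pawn driven by Enhanced Input, with controller-yaw-relative movement including vertical, controller yaw/pitch look, and bullet firing.
; BeginPlay adds the test mapping context and points RotatingMovement at ShieldRotationPivot.
; The shield input spawns ShieldNum evenly spaced shields in a ring around that pivot, attached so they orbit with it, then blocks respawning for a cooldown.
; An older four-shield layout and spring-arm pitch logic remain unconnected.
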(event Input|EnhancedActionEvents|EnhancedInputActionIA_TestShield
  (params (ActionValue :type Boolean) (ElapsedSeconds :type Float%20%28double-precision%29) (TriggeredSeconds :type Float%20%28double-precision%29) (InputAction :type Input%20Action%20Object%20Reference :default "/Game/Test/TestInput/IA_TestShield.IA_TestShield"))
  (bind _shield_rotation_pivot (Variables|Default|GetShield%20Rotation%20Pivot))
  (bind _disttoshield (Variables|Default|GetDistToShield))
  (:Started
    (if (Variables|Default|GetbCanSpawnShield)
      (Variables|Default|SetbCanSpawnShield false)
      (for _index (range 1 (Variables|Default|GetShieldNum))
        (bind _returnvalue (Game|SpawnActorfromClass "/Game/Test/TestBlueprint/BP_TestShield.BP_TestShield_C" (Math|Transform|MakeTransform (+ (Transformation|GetWorldLocation _shield_rotation_pivot) (* (Math|Vector|GetForwardVector _shield_rotation_pivot) (* _disttoshield (Math|Trig|Sin(Degrees) (Variables|Default|GetShieldDegree)))) (* (Math|Vector|GetRightVector _shield_rotation_pivot) (* _disttoshield (Math|Trig|Cos(Degrees) (Variables|Default|GetShieldDegree))))) (Math|Rotator|MakeRotator 0.0 0.0 (- 9e+01 (Variables|Default|GetShieldDegree)))) "Undefined" "MultiplyWithRoot" 0 0))
        (Transformation|AttachComponentToComponent _returnvalue (Variables|Default|GetShield%20Rotation%20Pivot) "None" "KeepWorld" "KeepRelative" "KeepRelative" true)
        (if (>= (+ (/ 3.6e+02 (Math|Conversions|ToFloat(Integer) (Variables|Default|GetShieldNum))) (Variables|Default|GetShieldDegree)) 3.6e+02)
          (Variables|Default|SetShieldDegree (- (+ (/ 3.6e+02 (Math|Conversions|ToFloat(Integer) (Variables|Default|GetShieldNum))) (Variables|Default|GetShieldDegree)) 3.6e+02))
          (else
            (Variables|Default|SetShieldDegree (+ (/ 3.6e+02 (Math|Conversions|ToFloat(Integer) (Variables|Default|GetShieldNum))) (Variables|Default|GetShieldDegree))))))
      (Utilities|FlowControl|Delay (Variables|Default|GetShieldCoolTime))
      (Variables|Default|SetbCanSpawnShield true))))

(event Input|EnhancedActionEvents|EnhancedInputActionIA_TestMove
  (params (ActionValue :type Vector :default "0, 0, 0") (ElapsedSeconds :type Float%20%28double-precision%29) (TriggeredSeconds :type Float%20%28double-precision%29) (InputAction :type Input%20Action%20Object%20Reference :default "/Game/Test/TestInput/IA_TestMove.IA_TestMove"))
  (bind _returnvalue (Pawn|GetController))
  (bind (_x _y _z) (Math|Vector|BreakVector ActionValue))
  (bind _returnvalue_2 (Transformation|GetActorRotation _returnvalue))
  (bind _returnvalue_3 (Math|Rotator|MakeRotator 0.0 0.0 (.yaw _returnvalue_2)))
  (Pawn|Input|AddMovementInput (+ (* (Math|Vector|GetForwardVector _returnvalue_3) _x) (* (Math|Vector|GetRightVector _returnvalue_3) _y) (* (Transformation|GetActorUpVector) _z)) 1.0 false))

(event Input|EnhancedActionEvents|EnhancedInputActionIA_TestFire
  (params (ActionValue :type Boolean) (ElapsedSeconds :type Float%20%28double-precision%29) (TriggeredSeconds :type Float%20%28double-precision%29) (InputAction :type Input%20Action%20Object%20Reference :default "/Game/Test/TestInput/IA_TestFire.IA_TestFire"))
  (:Started
    (Game|SpawnActorfromClass "/Game/Test/TestBlueprint/BP_TestBullet.BP_TestBullet_C" (Math|Transform|MakeTransform (+ (Transformation|GetActorLocation) (* (Transformation|GetActorForwardVector) 1e+02)) (Transformation|GetActorRotation) "1.000000,1.000000,1.000000") "Undefined" "MultiplyWithRoot" 0 0)))

(event Input|EnhancedActionEvents|EnhancedInputActionIA_TestRotation
  (params (ActionValue :type Vector%202D%20Structure) (ElapsedSeconds :type Float%20%28double-precision%29) (TriggeredSeconds :type Float%20%28double-precision%29) (InputAction :type Input%20Action%20Object%20Reference :default "/Game/Test/TestInput/IA_TestRotation.IA_TestRotation"))
  (bind (_x _y) (Math|Vector2D|BreakVector2D ActionValue))
  (Pawn|Input|AddControllerYawInput _x)
  ;[1 1 1] Spring Arm -> Use Pawn Control Rotation : true
  (bind _result (Math|Float|NegateFloat _y)
    (:%20%20
      (Pawn|Input|AddControllerPitchInput _result))))

(event EventBeginPlay
  (Utilities|FlowControl|Sequence
    (:then_0
      (bind _asplayer_controller (Utilities|Casting|CastToPlayerController (Pawn|GetController)))
      (Input|AddMappingContext (PlayerController|LocalPlayerSubsystems|GetEnhancedInputLocalPlayerSubsystem _asplayer_controller) "/Game/Test/TestInput/IMC_TestIMC.IMC_TestIMC" 0 "(bIgnoreAllPressedKeysUntilRelease=True,bForceImmediately=False,bNotifyUserSettings=False)"))
    (:then_1
      (Components|Movement|SetUpdatedComponent (Variables|Default|GetRotatingMovement) (Variables|Default|GetShield%20Rotation%20Pivot)))))

(event Collision|EventActorBeginOverlap
  (params (OtherActor :type Actor%20Object%20Reference)))

(event EventTick
  (params (DeltaSeconds :type Float%20%28single-precision%29)))

(fn ConstructionScript)